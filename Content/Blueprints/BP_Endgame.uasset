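; BP_Endgame is a trigger volume that plays the game's ending when a BP_Character overlaps its box.
; It disables the character's input, blends the view to EndGameCamera and turns on the point lights of all BP_EndgameLights actors.
; After a short delay it spawns a BP_EndgameMesh at a placed transform and calls its PlayAnimation.
; After a further configurable delay it opens the game-over level by name.
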(event `self.Box.OnComponentBeginOverlap`
  (params (OverlappedComponent :type "PrimitiveComponent Object Reference") (OtherActor :type "Actor Object Reference") (OtherComp :type "PrimitiveComponent Object Reference") (OtherBodyIndex :type Integer) (bFromSweep :type Boolean) (SweepResult :type "HitResult Structure (by ref)"))
  (bind _asbp_character (cast `/Game/Core/BP_Character` OtherActor))
  ;[1 1 1] Stop player
  (`self.DisableInput` _asbp_character (`GameplayStatics.GetPlayerController` 0))
  (`PlayerController.SetViewTargetWithBlend` (`GameplayStatics.GetPlayerController` 0) (`self.EndGameCamera`) 1.0 "VTBlend_Linear" 0.0 false)
  ;[1 1 1] Turn on lights
  (bind _outactors (`GameplayStatics.GetAllActorsOfClass` "/Game/Blueprints/BP_EndgameLights.BP_EndgameLights_C"))
  (for _array_element _outactors
    (`SceneComponent.SetVisibility` (`/Game/Blueprints/BP_EndgameLights.PointLight` _array_element) true false))
  ;[1 1 1] Spawn Endgame Mesh
  (`KismetSystemLibrary.Delay` 0.5)
  (bind _returnvalue (`|SpawnActorFromClass` "/Game/Blueprints/BP_EndgameMesh.BP_EndgameMesh_C" (`SceneComponent.K2_GetComponentToWorld` (`self.SpawnMeshTransform`)) "AlwaysSpawn" "OverrideRootScale" null null))
  (`/Game/Blueprints/BP_EndgameMesh.PlayAnimation` _returnvalue null 0.0)
  ;[1 1 1] GameOver
  (`KismetSystemLibrary.Delay` (`self.DelayBeforeGoToMenu`))
  (`GameplayStatics.OpenLevel` (`self.GameOverLevelName`)))

(fn `UserConstructionScript`)