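; BP_Goblin is an enemy character that chases the player on sight and makes a one-shot lunge attack.
; PawnSensing triggers FollowPlayer, which re-arms CanAttack and runs AI MoveTo toward the player.
; On arrival it calls a montage, waits briefly and debug-prints the distance to the seen pawn.
; If that pawn is out of range it resumes moving; otherwise it launches itself forward and up, then destroys itself.
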(event `self.PawnSensing.OnSeePawn`
  (params (Pawn :type "Pawn Object Reference"))
  (set `self.PlayerPawn` Pawn)
  (set `self.IsSeeingPlayer` true)
  (`self.FollowPlayer`))

(event `FollowPlayer`
  (bind _returnvalue (`KismetMathLibrary.VSize` (- (`self.K2_GetActorLocation` (`self.PlayerPawn`)) (`self.K2_GetActorLocation`))))
  (set `self.CanAttack` true)
  (if (`self.IsSeeingPlayer`)
    (`|AIMoveTo` self (0.0 0.0 0.0) (`GameplayStatics.GetPlayerCharacter` 0) 300.0 :!label _label
      (:`OnSuccess`
        (if (`self.CanAttack`)
          (set `self.CanAttack` false)
          (`self.PlayAnimMontage` null) ; Cambiar animacion de ataque
          (`KismetSystemLibrary.Delay` 0.5)
          (`KismetSystemLibrary.PrintText` (`KismetTextLibrary.Conv_DoubleToText` _returnvalue "HalfToEven"))
          (if (> _returnvalue 420.0)
            (goto _label)
            (else
              (`self.LaunchCharacter` (+ (* (`self.GetActorForwardVector`) (3000.0 3000.0 0.0)) (0.0 0.0 1000.0)))
              (`KismetSystemLibrary.Delay` 0.12)
              (`self.K2_DestroyActor`))))))))

(fn `UserConstructionScript`)