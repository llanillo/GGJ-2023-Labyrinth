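; BP_SplinePath is an obstacle Blueprint that moves a referenced actor along its spline, starting at BeginPlay.
; A timeline, with play rate set to the inverse of SplineMovementRate, drives an alpha lerped from zero to the spline's length.
; Each update sets the actor's world location at that distance and rotates it to face the spline tangent, without sweeping for collision.
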(event `self.ReceiveBeginPlay`
  (`TimelineComponent.SetPlayRate` (`self.MoveTimeline`) (/ 1.0 (`self.SplineMovementRate`)))
  (`self.StartMovementAlongSpline`))

(event `self.StartMovementAlongSpline`
  (`/Engine/EditorBlueprintResources/StandardMacros.IsValid` (`self.AActorToMoveAlongSpline`)
    (:`Is Valid`
      (bind (_direction _movetrack) (`Timeline|MoveTimeline` :!via `PlayFromStart`)
        (:`Update`
          (bind _returnvalue (`KismetMathLibrary.Lerp` 0.0 (`SplineComponent.GetSplineLength` (`self.SplineComponent`)) _movetrack))
          (`self.K2_SetActorLocation` (`self.AActorToMoveAlongSpline`) (`SplineComponent.GetLocationAtDistanceAlongSpline` (`self.SplineComponent`) _returnvalue "World") false false)
          (`self.K2_SetActorRotation` (`self.AActorToMoveAlongSpline`) (`KismetMathLibrary.Conv_VectorToRotator` (`SplineComponent.GetTangentAtDistanceAlongSpline` (`self.SplineComponent`) _returnvalue "World")) false))))))

(fn `UserConstructionScript`)